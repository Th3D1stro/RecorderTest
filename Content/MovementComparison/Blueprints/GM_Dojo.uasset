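; GM_Dojo is the dojo game mode for movement comparison, which bootstraps the movement cache and training controller actors.
; After a short BeginPlay delay, SafeSpawnControllerAndCache spawns both classes at the world origin, ignoring collisions, and stores valid references.
; Failed spawns print a "class not set" message.
; The function also sets local validity flags, but its combined return is unconnected and never runs.
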(event `self.ReceiveBeginPlay`
  (`KismetSystemLibrary.Delay` 0.05)
  (`self.SafeSpawnControllerAndCache` self))

(event `self.ReceiveTick`
  (params (DeltaSeconds :type "Float (single-precision)")))

(fn `SafeSpawnControllerAndCache`
  (returns (bSuccess :type Boolean))
  (bind _returnvalue (`KismetMathLibrary.MakeTransform` (0.0 0.0 0.0)))
  (`|ExecutionSequence`
    (:`then_0`
      (bind _returnvalue_2 (`|SpawnActorFromClass` (`self.MovementCacheClass`) _returnvalue "AlwaysSpawn" "SelectDefaultAtRuntime" null null))
      (bind _returnvalue_3 (`|SpawnActorFromClass` (`self.TrainingControllerClass`) _returnvalue "AlwaysSpawn" "SelectDefaultAtRuntime" null null))
      (`|ExecutionSequence`
        (:`then_0`
          (`/Engine/EditorBlueprintResources/StandardMacros.IsValid` _returnvalue_2
            (:`Is Valid`
              (set `self.MovementCacheRef` _returnvalue_2))
            (:`Is Not Valid`
              (`KismetSystemLibrary.PrintString` "[GM] MovementCacheClass not set"))))
        (:`then_1`
          (`/Engine/EditorBlueprintResources/StandardMacros.IsValid` _returnvalue_3
            (:`Is Valid`
              (set `self.TrainingControllerRef` _returnvalue_3))
            (:`Is Not Valid`
              (`KismetSystemLibrary.PrintString` "[GM] TrainingControllerClass not set"))))))
    (:`then_1`
      (`/Engine/EditorBlueprintResources/StandardMacros.IsValid` (`self.MovementCacheRef`)
        (:`Is Valid`
          (set `self.Local_CacheValid` true))
        (:`Is Not Valid`
          (set `self.Local_CacheValid` false))))
    (:`then_2`
      (`/Engine/EditorBlueprintResources/StandardMacros.IsValid` (`self.TrainingControllerRef`)
        (:`Is Valid`
          (set `self.Local_ControllerValid` true))
        (:`Is Not Valid`
          (set `self.Local_ControllerValid` false))))))

(fn `UserConstructionScript`)