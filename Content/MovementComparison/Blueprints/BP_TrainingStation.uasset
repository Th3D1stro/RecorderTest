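; BP_TrainingStation is an actor in the MovementComparison area that manages a set of widget component panels, such as main menu, movement list, start panel, HUD and results.
; HideAllPanels runs on BeginPlay, turning off visibility and collision for every panel.
; ShowOnlyPanel hides all, then enables one by name with query-only collision, while GetWidgetForPanel returns its user widget.
; PhaseResult and FinalResult panels are only hidden, absent from both name lookups.
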(event `self.ReceiveBeginPlay`
  (`self.HideAllPanels`))

(event `self.ReceiveActorBeginOverlap`
  (params (OtherActor :type "Actor Object Reference")))

(event `self.ReceiveTick`
  (params (DeltaSeconds :type "Float (single-precision)")))

(fn `GetWidgetForPanel`
  (params (PanelName :type Name))
  (returns (Widget :type "UserWidget Object Reference"))
  (if (== PanelName "MainMenu")
    (return (`WidgetComponent.GetUserWidgetObject` (`self.WidgetComp_MainMenu`)))
    (elif (== PanelName "MovementList")
      (return (`WidgetComponent.GetUserWidgetObject` (`self.WidgetComp_MovementList`)))
      (elif (== PanelName "StartPanel")
        (return (`WidgetComponent.GetUserWidgetObject` (`self.WidgetComp_StartPanel`)))
        (elif (== PanelName "HUD")
          (return (`WidgetComponent.GetUserWidgetObject` (`self.WidgetComp_HUD`)))
          (elif (== PanelName "Results")
            (return (`WidgetComponent.GetUserWidgetObject` (`self.WidgetComp_Results`)))
            (else
              (return null))))))))

(fn `HideAllPanels`
  (bind _widgetcomp_mainmenu (`self.WidgetComp_MainMenu`))
  (bind _widgetcomp_movementlist (`self.WidgetComp_MovementList`))
  (bind _widgetcomp_startpanel (`self.WidgetComp_StartPanel`))
  (bind _widgetcomp_hud (`self.WidgetComp_HUD`))
  (bind _widgetcomp_phaseresult (`self.WidgetComp_PhaseResult`))
  (bind _widgetcomp_finalresult (`self.WidgetComp_FinalResult`))
  (bind _widgetcomp_results (`self.WidgetComp_Results`))
  (`SceneComponent.SetVisibility` _widgetcomp_mainmenu false false)
  (`PrimitiveComponent.SetCollisionEnabled` _widgetcomp_mainmenu "NoCollision")
  (`SceneComponent.SetVisibility` _widgetcomp_movementlist false false)
  (`PrimitiveComponent.SetCollisionEnabled` _widgetcomp_movementlist "NoCollision")
  (`SceneComponent.SetVisibility` _widgetcomp_startpanel false false)
  (`PrimitiveComponent.SetCollisionEnabled` _widgetcomp_startpanel "NoCollision")
  (`SceneComponent.SetVisibility` _widgetcomp_hud false false)
  (`PrimitiveComponent.SetCollisionEnabled` _widgetcomp_hud "NoCollision")
  (`SceneComponent.SetVisibility` _widgetcomp_phaseresult false false)
  (`PrimitiveComponent.SetCollisionEnabled` _widgetcomp_phaseresult "NoCollision")
  (`SceneComponent.SetVisibility` _widgetcomp_finalresult false false)
  (`PrimitiveComponent.SetCollisionEnabled` _widgetcomp_finalresult "NoCollision")
  (`SceneComponent.SetVisibility` _widgetcomp_results false false)
  (`PrimitiveComponent.SetCollisionEnabled` _widgetcomp_results "NoCollision"))

(fn `ShowOnlyPanel`
  (params (PanelName :type Name))
  (`self.HideAllPanels`)
  (if (== PanelName "MainMenu")
    (`SceneComponent.SetVisibility` (`self.WidgetComp_MainMenu`) true false)
    (`PrimitiveComponent.SetCollisionEnabled` (`self.WidgetComp_MainMenu`) "QueryOnly")
    (elif (== PanelName "MovementList")
      (`SceneComponent.SetVisibility` (`self.WidgetComp_MovementList`) true false)
      (`PrimitiveComponent.SetCollisionEnabled` (`self.WidgetComp_MovementList`) "QueryOnly")
      (elif (== PanelName "StartPanel")
        (`SceneComponent.SetVisibility` (`self.WidgetComp_StartPanel`) true false)
        (`PrimitiveComponent.SetCollisionEnabled` (`self.WidgetComp_StartPanel`) "QueryOnly")
        (elif (== PanelName "HUD")
          (`SceneComponent.SetVisibility` (`self.WidgetComp_HUD`) true false)
          (`PrimitiveComponent.SetCollisionEnabled` (`self.WidgetComp_HUD`) "QueryOnly")
          (elif (== PanelName "Results")
            (`SceneComponent.SetVisibility` (`self.WidgetComp_Results`) true false)
            (`PrimitiveComponent.SetCollisionEnabled` (`self.WidgetComp_Results`) "QueryOnly")))))))

(fn `UserConstructionScript`)