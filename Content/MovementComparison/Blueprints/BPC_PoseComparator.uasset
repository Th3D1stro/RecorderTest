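; Pose-scoring component for movement training that compares a VR user's body pose against a guide's.
; EvaluateOnce reads the guide via BPI_PoseProvider and the user's IK transforms, then sends per-tracker feedback to the owning BP_TrainingController.
; Knees and elbows score by joint-angle plus waist-relative direction error in degrees, despite the ThresholdCm naming; six other trackers always pass.
; BuildPhaseResult packages average score, reaction time and failed trackers.
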(event EventBeginPlay)

(event EventTick
  (params (DeltaSeconds :type Float%20%28single-precision%29)))

(fn StartEvaluation
  (params (InGuide :type Actor%20Object%20Reference) (InUser :type Actor%20Object%20Reference) (PhaseIndex :type Integer) (DurationSec :type Float%20%28single-precision%29) (ThresholdOverrideCm :type Float%20%28single-precision%29))
  (bind _returnvalue (Class|KismetSystemLibrary|MakeLiteralBool true))
  (Utilities|IsValid InGuide
    (:Is%20Valid
      (Utilities|IsValid InUser
        (:Is%20Valid
          (Variables|Comparator|Refs|SetGuideRef InGuide)
          (Variables|Comparator|Refs|SetUserRef InUser)
          (Variables|Comparator|State|SetCurrentPhaseIndex PhaseIndex)
          (Variables|Default|SetCurrentEvaluationDuration DurationSec)
          (Variables|Comparator|State|SetbIsEvaluating _returnvalue)
          (Variables|Default|SetEvaluationStartTime (Utilities|Time|GetGameTimeinSeconds))
          (Variables|Default|SetFirstCorrectTime (Math|Float|MakeLiteralFloat -1.0))
          (Variables|Default|SetSum (Math|Float|MakeLiteralFloat 0.0))
          (Variables|Comparator|Internal|SetCompare_CorrectCount (Class|KismetSystemLibrary|MakeLiteralInteger))
          (Utilities|Array|Clear (Variables|Comparator|State|GetCurrentScores))
          (Utilities|Array|Clear (Variables|Comparator|State|GetTrackersFailedAccum))
          (Utilities|Array|Clear (Variables|Comparator|Internal|GetCompareTwoPoses_Results))
          (if (> ThresholdOverrideCm (Math|Float|MakeLiteralFloat 0.0))
            (Variables|Comparator|Settings|SetThresholdCm ThresholdOverrideCm)
            (return _returnvalue)
            (else
              (return _returnvalue))))
        (:Is%20Not%20Valid
          (return (Class|KismetSystemLibrary|MakeLiteralBool false)))))
    (:Is%20Not%20Valid
      (return (Class|KismetSystemLibrary|MakeLiteralBool false)))))

(fn StopEvaluation)

(fn EvaluateOnce
  (bind (_outpose _bvalid) (CallFunction|SafeGetGuidePose))
  (Development|PrintString (Utilities|String|Append "GuideValid=" (Utilities|String|ToString(Boolean) _bvalid)) true false "(R=0.000000,G=1.000000,B=1.000000,A=1.000000)")
  (bind (_outpose_2 _bvalid_2) (CallFunction|SafeGetUserPose))
  (Development|PrintString (Utilities|String|Append "UserValid=" (Utilities|String|ToString(Boolean) _bvalid_2)) true false "(R=1.000000,G=0.000000,B=1.000000,A=1.000000)")
  (if (and _bvalid _bvalid_2)
    (bind _instantscore01 (CallFunction|CompareTwoPoses _outpose _outpose_2 (Variables|Comparator|Settings|GetThresholdCm)))
    (for _array_element (Variables|Comparator|Internal|GetCompareTwoPoses_Results)
      (bind _asbp_training_controller (Utilities|Casting|CastToBP_TrainingController (Components|GetOwner)))
      (Default|ShowTrackerFeedback _asbp_training_controller (.TrackerName (Utilities|Struct|BreakS_TrackerEvalResult _array_element)) (.bWithinThreshold (Utilities|Struct|BreakS_TrackerEvalResult _array_element)) (Math|Vector|MakeVector 0.0 0.0 0.0)))
    (return _instantscore01 (Variables|Comparator|Internal|GetCompareTwoPoses_Results))
    (else
      (Development|PrintString "ELSE BRANCH HIT (score forced to 0)" true false "(R=1.000000,G=0.000000,B=0.000000,A=1.000000)")
      (Utilities|Array|Clear (Variables|Comparator|Internal|GetCompareTwoPoses_Results))
      (return (Math|Float|MakeLiteralFloat 0.0) (Variables|Comparator|Internal|GetCompareTwoPoses_Results)))))

(fn BuildPhaseResult
  (bind _currentscores (Variables|Comparator|State|GetCurrentScores))
  (bind _firstcorrecttime (Variables|Default|GetFirstCorrectTime))
  (bind _returnvalue (Utilities|Array|Length _currentscores))
  (Variables|Comparator|Internal|SetBuildPhase_Sum 0.0)
  (for _array_element (Variables|Comparator|State|GetCurrentScores)
    (Variables|Comparator|Internal|SetBuildPhase_Sum (+ (Variables|Comparator|Internal|GetBuildPhase_Sum) _array_element)))
  (return (Utilities|Struct|MakeS_PhaseResult (Variables|Comparator|State|GetCurrentPhaseIndex) "" (select (> _returnvalue 0) (/ (Variables|Comparator|Internal|GetBuildPhase_Sum) _returnvalue) (Math|Float|MakeLiteralFloat 0.0)) (select (> _firstcorrecttime 0.0) _firstcorrecttime (Variables|Default|GetCurrentEvaluationDuration)) (Variables|Comparator|State|GetCurrentScores) (Variables|Comparator|State|GetTrackersFailedAccum) true)))

(fn SafeGetUserPose
  (bind _userref (Variables|Comparator|Refs|GetUserRef))
  (Utilities|IsValid _userref
    (:Is%20Valid
      (bind _asvr_character_bp (Utilities|Casting|CastToVR_CharacterBP _userref)
        (:then
          (return (Utilities|Struct|MakeS_GuidePoseFrame (Utilities|Time|GetGameTimeinSeconds) true (Variables|/Game/Players/Player_Level2/VR_CharacterBP.VR_CharacterBP_C|GetIK_Waist _asvr_character_bp) (Variables|/Game/Players/Player_Level2/VR_CharacterBP.VR_CharacterBP_C|GetIK_LeftKnee _asvr_character_bp) (Variables|/Game/Players/Player_Level2/VR_CharacterBP.VR_CharacterBP_C|GetIK_RightKnee _asvr_character_bp) (Variables|/Game/Players/Player_Level2/VR_CharacterBP.VR_CharacterBP_C|GetIK_LeftFoot _asvr_character_bp) (Variables|/Game/Players/Player_Level2/VR_CharacterBP.VR_CharacterBP_C|GetIK_RightFoot _asvr_character_bp) (Variables|/Game/Players/Player_Level2/VR_CharacterBP.VR_CharacterBP_C|GetIK_LeftElbow _asvr_character_bp) (Variables|/Game/Players/Player_Level2/VR_CharacterBP.VR_CharacterBP_C|GetIK_RightElbow _asvr_character_bp) (Variables|/Game/Players/Player_Level2/VR_CharacterBP.VR_CharacterBP_C|GetIK_Head _asvr_character_bp) (Variables|/Game/Players/Player_Level2/VR_CharacterBP.VR_CharacterBP_C|GetIK_LeftHand _asvr_character_bp) (Variables|/Game/Players/Player_Level2/VR_CharacterBP.VR_CharacterBP_C|GetIK_RightHand _asvr_character_bp)) true))
        (:CastFailed
          (return (Utilities|Struct|MakeS_GuidePoseFrame 0.0 false) false))))
    (:Is%20Not%20Valid
      (return (Utilities|Struct|MakeS_GuidePoseFrame 0.0 false) false))))

(fn SafeGetGuidePose
  (bind _s_guideposeframe (Utilities|Struct|MakeS_GuidePoseFrame 0.0 false))
  (bind _guideref (Variables|Comparator|Refs|GetGuideRef))
  (Utilities|IsValid _guideref
    (:Is%20Valid
      (if (Utilities|DoesObjectImplementInterface _guideref "/Game/MovementComparison/Interfaces/BPI_PoseProvider.BPI_PoseProvider_C")
        (bind (_outpose _bisvalid) (Class|BPIPoseProvider|GetCurrentPose(Message) _guideref))
        (return _outpose _bisvalid)
        (else
          (return _s_guideposeframe false))))
    (:Is%20Not%20Valid
      (return _s_guideposeframe false))))

(fn CompareTwoPoses
  (params (GuidePose :type S%20Guide%20Pose%20Frame%20Structure) (UserPose :type S%20Guide%20Pose%20Frame%20Structure) (ThresholdCm :type Float%20%28single-precision%29))
  (bind (_timestamp _bvalid _ik_waist _ik_leftknee _ik_rightknee _ik_leftfoot _ik_rightfoot _ik_leftelbow _ik_rightelbow _ik_head _ik_lefthand _ik_righthand) (Utilities|Struct|BreakS_GuidePoseFrame GuidePose))
  (bind (_timestamp_2 _bvalid_2 _ik_waist_2 _ik_leftknee_2 _ik_rightknee_2 _ik_leftfoot_2 _ik_rightfoot_2 _ik_leftelbow_2 _ik_rightelbow_2 _ik_head_2 _ik_lefthand_2 _ik_righthand_2) (Utilities|Struct|BreakS_GuidePoseFrame UserPose))
  (bind _location (Math|Transform|BreakTransform _ik_waist))
  (bind _location_2 (Math|Transform|BreakTransform _ik_leftelbow))
  (bind _location_3 (Math|Transform|BreakTransform _ik_leftelbow_2))
  (bind _location_4 (Math|Transform|BreakTransform _ik_rightelbow))
  (bind _location_5 (Math|Transform|BreakTransform _ik_rightelbow_2))
  (bind _location_6 (Math|Transform|BreakTransform _ik_leftknee))
  (bind _location_7 (Math|Transform|BreakTransform _ik_waist_2))
  (bind _location_8 (Math|Transform|BreakTransform _ik_leftknee_2))
  (bind _location_9 (Math|Transform|BreakTransform _ik_rightknee))
  (bind _location_10 (Math|Transform|BreakTransform _ik_rightknee_2))
  (Utilities|FlowControl|Sequence
    (:then_0
      (Variables|Comparator|Internal|SetCompare_CorrectCount 0)
      (Utilities|Array|Clear (Variables|Comparator|Internal|GetCompareTwoPoses_Results)))
    (:then_1
      (Utilities|FlowControl|Sequence
        (:then_0
          (bind _angledegrees (CallFunction|CalculateJointAngle _location _location_6 (.Location (Math|Transform|BreakTransform _ik_leftfoot))))
          (bind _angledegrees_2 (CallFunction|CalculateJointAngle _location_7 _location_8 (.Location (Math|Transform|BreakTransform _ik_leftfoot_2))))
          (Utilities|Array|Add (Variables|Comparator|Internal|GetCompareTwoPoses_Results) (Utilities|Struct|MakeS_TrackerEvalResult (Utilities|Enum|LiteralenumE_TrackerName "NewEnumerator1") (+ (Math|Float|Absolute(Float) (- _angledegrees _angledegrees_2)) (CallFunction|CalculateVectorDeviation _location _location_6 _location_7 _location_8)) (<= (+ (Math|Float|Absolute(Float) (- _angledegrees _angledegrees_2)) (CallFunction|CalculateVectorDeviation _location _location_6 _location_7 _location_8)) ThresholdCm) true))
          (if (<= (+ (Math|Float|Absolute(Float) (- _angledegrees _angledegrees_2)) (CallFunction|CalculateVectorDeviation _location _location_6 _location_7 _location_8)) ThresholdCm)
            (Variables|Comparator|Internal|SetCompare_CorrectCount (stale _result))))
        (:then_1
          (bind _angledegrees_3 (CallFunction|CalculateJointAngle _location _location_9 (.Location (Math|Transform|BreakTransform _ik_rightfoot))))
          (bind _angledegrees_4 (CallFunction|CalculateJointAngle _location_7 _location_10 (.Location (Math|Transform|BreakTransform _ik_rightfoot_2))))
          (Utilities|Array|Add (Variables|Comparator|Internal|GetCompareTwoPoses_Results) (Utilities|Struct|MakeS_TrackerEvalResult (Utilities|Enum|LiteralenumE_TrackerName "NewEnumerator2") (+ (Math|Float|Absolute(Float) (- _angledegrees_3 _angledegrees_4)) (CallFunction|CalculateVectorDeviation _location _location_9 _location_7 _location_10)) (<= (+ (Math|Float|Absolute(Float) (- _angledegrees_3 _angledegrees_4)) (CallFunction|CalculateVectorDeviation _location _location_9 _location_7 _location_10)) ThresholdCm) true))
          (if (<= (+ (Math|Float|Absolute(Float) (- _angledegrees_3 _angledegrees_4)) (CallFunction|CalculateVectorDeviation _location _location_9 _location_7 _location_10)) ThresholdCm)
            (Variables|Comparator|Internal|SetCompare_CorrectCount (stale _result))))
        (:then_2
          (bind _angledegrees_5 (CallFunction|CalculateJointAngle _location _location_2 (.Location (Math|Transform|BreakTransform _ik_lefthand))))
          (bind _angledegrees_6 (CallFunction|CalculateJointAngle _location_7 _location_3 (.Location (Math|Transform|BreakTransform _ik_lefthand_2))))
          (Utilities|Array|Add (Variables|Comparator|Internal|GetCompareTwoPoses_Results) (Utilities|Struct|MakeS_TrackerEvalResult (Utilities|Enum|LiteralenumE_TrackerName "NewEnumerator5") (+ (Math|Float|Absolute(Float) (- _angledegrees_5 _angledegrees_6)) (CallFunction|CalculateVectorDeviation _location _location_2 _location_7 _location_3)) (<= (+ (Math|Float|Absolute(Float) (- _angledegrees_5 _angledegrees_6)) (CallFunction|CalculateVectorDeviation _location _location_2 _location_7 _location_3)) ThresholdCm) true))
          (if (<= (+ (Math|Float|Absolute(Float) (- _angledegrees_5 _angledegrees_6)) (CallFunction|CalculateVectorDeviation _location _location_2 _location_7 _location_3)) ThresholdCm)
            (Variables|Comparator|Internal|SetCompare_CorrectCount (stale _result))))
        (:then_3
          (bind _angledegrees_7 (CallFunction|CalculateJointAngle _location _location_4 (.Location (Math|Transform|BreakTransform _ik_righthand))))
          (bind _angledegrees_8 (CallFunction|CalculateJointAngle _location_7 _location_5 (.Location (Math|Transform|BreakTransform _ik_righthand_2))))
          (Utilities|Array|Add (Variables|Comparator|Internal|GetCompareTwoPoses_Results) (Utilities|Struct|MakeS_TrackerEvalResult (Utilities|Enum|LiteralenumE_TrackerName "NewEnumerator6") (+ (Math|Float|Absolute(Float) (- _angledegrees_7 _angledegrees_8)) (CallFunction|CalculateVectorDeviation _location _location_4 _location_7 _location_5)) (<= (+ (Math|Float|Absolute(Float) (- _angledegrees_7 _angledegrees_8)) (CallFunction|CalculateVectorDeviation _location _location_4 _location_7 _location_5)) ThresholdCm) true))
          (if (<= (+ (Math|Float|Absolute(Float) (- _angledegrees_7 _angledegrees_8)) (CallFunction|CalculateVectorDeviation _location _location_4 _location_7 _location_5)) ThresholdCm)
            (Variables|Comparator|Internal|SetCompare_CorrectCount (stale _result))))
        (:then_4
          (Utilities|Array|Add (Variables|Comparator|Internal|GetCompareTwoPoses_Results) (Utilities|Struct|MakeS_TrackerEvalResult (Utilities|Enum|LiteralenumE_TrackerName "NewEnumerator0") (Math|Float|MakeLiteralFloat 0.0) true true))
          (Variables|Comparator|Internal|SetCompare_CorrectCount (stale _result)))
        (:then_5
          (Utilities|Array|Add (Variables|Comparator|Internal|GetCompareTwoPoses_Results) (Utilities|Struct|MakeS_TrackerEvalResult (Utilities|Enum|LiteralenumE_TrackerName "NewEnumerator3") (Math|Float|MakeLiteralFloat 0.0) true true))
          (Variables|Comparator|Internal|SetCompare_CorrectCount (stale _result)))
        (:then_6
          (Utilities|Array|Add (Variables|Comparator|Internal|GetCompareTwoPoses_Results) (Utilities|Struct|MakeS_TrackerEvalResult (Utilities|Enum|LiteralenumE_TrackerName "NewEnumerator4") (Math|Float|MakeLiteralFloat 0.0) true true))
          (Variables|Comparator|Internal|SetCompare_CorrectCount (stale _result)))
        (:then_7
          (Utilities|Array|Add (Variables|Comparator|Internal|GetCompareTwoPoses_Results) (Utilities|Struct|MakeS_TrackerEvalResult (Utilities|Enum|LiteralenumE_TrackerName "NewEnumerator7") (Math|Float|MakeLiteralFloat 0.0) true true))
          (Variables|Comparator|Internal|SetCompare_CorrectCount (stale _result)))
        (:then_8
          (Utilities|Array|Add (Variables|Comparator|Internal|GetCompareTwoPoses_Results) (Utilities|Struct|MakeS_TrackerEvalResult (Utilities|Enum|LiteralenumE_TrackerName "NewEnumerator8") (Math|Float|MakeLiteralFloat 0.0) true true))
          (Variables|Comparator|Internal|SetCompare_CorrectCount (stale _result)))
        (:then_9
          (Utilities|Array|Add (Variables|Comparator|Internal|GetCompareTwoPoses_Results) (Utilities|Struct|MakeS_TrackerEvalResult (Utilities|Enum|LiteralenumE_TrackerName "NewEnumerator9") (Math|Float|MakeLiteralFloat 0.0) true true))
          (Variables|Comparator|Internal|SetCompare_CorrectCount (stale _result)))))
    (:then_2
      (return (Variables|Comparator|Internal|GetCompareTwoPoses_Results) (Math|Float|SafeDivide (Math|Conversions|ToFloat(Integer) (Variables|Comparator|Internal|GetCompare_CorrectCount)) (Math|Float|MakeLiteralFloat 1e+01))))))

(fn ResetEvaluationState
  (Utilities|Array|Clear (Variables|Comparator|State|GetCurrentScores))
  (Utilities|Array|Clear (Variables|Comparator|State|GetTrackersFailedAccum))
  (Variables|Default|SetFirstCorrectTime -1.0)
  (Variables|Default|SetEvaluationStartTime 0.0)
  (Variables|Comparator|State|SetbIsEvaluating false)
  (Utilities|Time|ClearandInvalidateTimerbyHandle (Variables|Comparator|State|GetEvalTimerHandle)))

(fn CalculateJointAngle
  (params (RootPoint :type Vector) (HingePoint :type Vector) (EndPoint :type Vector))
  (return (Class|KismetMathLibrary|DegAcos (Math|Vector|DotProduct (Math|Vector|GetUnitDirection(Vector) HingePoint RootPoint) (Math|Vector|GetUnitDirection(Vector) HingePoint EndPoint)))))

(fn CalculateVectorDeviation
  (params (GuideStart :type Vector) (GuideEnd :type Vector) (UserStart :type Vector) (UserEnd :type Vector))
  (return (Class|KismetMathLibrary|DegAcos (Math|Vector|DotProduct (Math|Vector|GetUnitDirection(Vector) GuideStart GuideEnd) (Math|Vector|GetUnitDirection(Vector) UserStart UserEnd)))))