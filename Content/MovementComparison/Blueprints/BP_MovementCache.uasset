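; BP_MovementCache preloads recorded movement snapshots from save games and serves them from memory by slot name.
; On BeginPlay, WarmUp runs once, walking MovementsTable rows and loading each SaveSlotName through LoadOneSlot, which validates existence, class and a snapshot count limit.
; Successful loads fill the SnapshotsBySlot map for GetSnapshots and HasSnapshots, while failures are counted or logged.
; ClearCache, ReloadSlot and GetCachedSlotNames are unimplemented stubs.
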(event `self.ReceiveBeginPlay`
  (bind (_numloaded _numfailed) (`self.WarmUp`))
  (`KismetSystemLibrary.PrintString` (`KismetStringLibrary.Concat_StrStr` (`KismetStringLibrary.Concat_StrStr` (`KismetStringLibrary.Concat_StrStr` "[Cache] BeginPlay WarmUp -> Loaded=" (`KismetStringLibrary.Conv_IntToString` _numloaded)) " Failed=") (`KismetStringLibrary.Conv_IntToString` _numfailed))))

(event `self.ReceiveActorBeginOverlap`
  (params (OtherActor :type "Actor Object Reference")))

(event `self.ReceiveTick`
  (params (DeltaSeconds :type "Float (single-precision)")))

(fn `ClearCache`)

(fn `GetCachedSlotNames`
  (returns (OutNames :type "Array of Name"))
  (return))

(fn `GetSnapshots`
  (params (SlotName :type Name))
  (returns (bSuccess :type Boolean) (OutSnapshots :type "Array of /Game/Data/Recorder/Struct/S_TrackerSnapshot Structure"))
  (bind (_value _returnvalue) (`BlueprintMapLibrary.Map_Find` (`self.SnapshotsBySlot`) SlotName))
  (if _returnvalue
    (return _returnvalue (`.Snapshots_2_AC16D2DE424D32DE2E4C17A2E2EF17A2` (break `/Game/MovementComparison/Structs/S_SnapshotArray` _value)))
    (else
      (return _returnvalue))))

(fn `HasSnapshots`
  (params (SlotName :type Name))
  (returns (bExists :type Boolean))
  (return (`BlueprintMapLibrary.Map_Contains` (`self.SnapshotsBySlot`) SlotName)))

(fn `LoadOneSlot`
  (params (SlotName :type String))
  (returns (bSuccess :type Boolean) (OutSnapshots :type "Array of /Game/Data/Recorder/Struct/S_TrackerSnapshot Structure"))
  (bind _returnvalue (`GameplayStatics.DoesSaveGameExist` SlotName))
  (if _returnvalue
    (bind _returnvalue_2 (`GameplayStatics.LoadGameFromSlot` SlotName))
    (`/Engine/EditorBlueprintResources/StandardMacros.IsValid` _returnvalue_2
      (:`Is Valid`
        (bind _asbp_movement_save_game (cast `/Game/Data/Recorder/SaveGame/BP_MovementSaveGame` _returnvalue_2)
          (:`then`
            (bind _recordedsnapshots (`/Game/Data/Recorder/SaveGame/BP_MovementSaveGame.RecordedSnapshots` _asbp_movement_save_game))
            (bind _returnvalue_3 (`KismetArrayLibrary.Array_Length` _recordedsnapshots))
            (if (> _returnvalue_3 (`self.MaxSnapshotsPerSlotSafety`))
              (bind _output_get (set `self.LastError` (`KismetStringLibrary.Concat_StrStr` "[Cache] Too many snapshots: " SlotName)))
              (`KismetSystemLibrary.PrintString` _output_get)
              (return false)
              (else
                (`KismetSystemLibrary.PrintString` (`KismetStringLibrary.Concat_StrStr` (`KismetStringLibrary.Concat_StrStr` (`KismetStringLibrary.Concat_StrStr` (`KismetStringLibrary.Concat_StrStr` "[Cache] Loaded " SlotName) " with ") (`KismetStringLibrary.Conv_IntToString` _returnvalue_3)) " snapshots"))
                (return true _recordedsnapshots))))
          (:`CastFailed`
            (bind _output_get_2 (set `self.LastError` (`KismetStringLibrary.Concat_StrStr` "[Cache] Cast failed: " SlotName)))
            (`KismetSystemLibrary.PrintString` _output_get_2)
            (return false))))
      (:`Is Not Valid`
        (bind _output_get_3 (set `self.LastError` (`KismetStringLibrary.Concat_StrStr` "[Cache] Failed to load: " SlotName)))
        (`KismetSystemLibrary.PrintString` _output_get_3)
        (return false)))
    (else
      (bind _output_get_4 (set `self.LastError` (`KismetStringLibrary.Concat_StrStr` "[Cache] Slot not found: " SlotName)))
      (`KismetSystemLibrary.PrintString` _output_get_4)
      (return false))))

(fn `ReloadSlot`
  (params (SlotName :type Name))
  (returns (bSuccess :type Boolean))
  (return false))

(fn `UserConstructionScript`)

(fn `WarmUp`
  (returns (NumLoaded :type Integer) (NumFailed :type Integer))
  (bind _movementstable (`self.MovementsTable`))
  (bind _warmup_localnumloaded (`self.WarmUp_LocalNumLoaded`))
  (bind _warmup_localnumfailed (`self.WarmUp_LocalNumFailed`))
  (set `self.WarmUp_LocalNumLoaded` 0)
  (set `self.WarmUp_LocalNumFailed` 0)
  (if (`self.bWarmedUp`)
    (return 0 0)
    (else
      (`/Engine/EditorBlueprintResources/StandardMacros.IsValid` _movementstable
        (:`Is Valid`
          (bind _outrownames (`DataTableFunctionLibrary.GetDataTableRowNames` _movementstable))
          (for _array_element _outrownames
            (bind _returnvalue (`|GetDataTableRow` _movementstable _array_element)
              (:`then`
                (bind (_movementname _category _saveslotname) (break `/Game/MovementComparison/Structs/S_MovementInfo` _returnvalue))
                (if (`KismetStringLibrary.EqualEqual_StrStr` _saveslotname)
                  (set `self.WarmUp_LocalNumFailed` (+ (`self.WarmUp_LocalNumFailed`) 1))
                  (else
                    (bind (_bsuccess _outsnapshots) (`self.LoadOneSlot` _saveslotname))
                    (if _bsuccess
                      (`BlueprintMapLibrary.Map_Add` (`self.SnapshotsBySlot`) (`KismetStringLibrary.Conv_StringToName` _saveslotname) (make `/Game/MovementComparison/Structs/S_SnapshotArray` _outsnapshots))
                      (set `self.WarmUp_LocalNumLoaded` (+ (`self.WarmUp_LocalNumLoaded`) 1))
                      (else
                        (set `self.WarmUp_LocalNumFailed` (+ (`self.WarmUp_LocalNumFailed`) 1)))))))
              (:`RowNotFound`
                (set `self.WarmUp_LocalNumFailed` (+ (`self.WarmUp_LocalNumFailed`) 1)))))
          (set `self.bWarmedUp` true)
          (`KismetSystemLibrary.PrintString` (`KismetStringLibrary.Concat_StrStr` (`KismetStringLibrary.Concat_StrStr` (`KismetStringLibrary.Concat_StrStr` "[Cache] Loaded " (`KismetStringLibrary.Conv_IntToString` _warmup_localnumloaded)) " / Failed ") (`KismetStringLibrary.Conv_IntToString` _warmup_localnumfailed)))
          (return _warmup_localnumloaded _warmup_localnumfailed))
        (:`Is Not Valid`
          (set `self.LastError` "[Cache] No DataTable assigned")
          (`KismetSystemLibrary.PrintString` "[Cache] No DataTable assigned")
          (return 0 0))))))