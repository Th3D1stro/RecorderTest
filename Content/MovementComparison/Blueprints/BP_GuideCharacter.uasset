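; Guide character that holds teacher full-body IK pose sequences for movement comparison.
; LoadMovementFromCache fills TeacherPoses from a procedural DataTable row named by save slot, falling back to cached tracker snapshots.
; GetInterpolatedSnapshot lerps bracketing keyframes, but samples at a fixed time zero rather than PlaybackTime.
; GetCurrentPose packages the IK variables, while playback, IK application, pole vectors and student evaluation are stubs.
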(event `self.ReceiveBeginPlay`)

(event `self.ReceiveActorBeginOverlap`
  (params (OtherActor :type "Actor Object Reference")))

(fn `ApplySnapshotToIK`)

(fn `BuildCurrentPoseFrame`)

(fn `ComputeAndApplyPoleVectors`)

(fn `EvaluateStudentPose`
  (locals (LocalMinError :type "Float (double-precision)" :default 999.0) (LocalBestIndex :type Integer) (LocalLastIndex :type Integer) (LocalUserPose :type "/Game/MovementComparison/Structs/S_GuidePoseFrame Structure") (LocalIterError :type "Float (double-precision)") (LocalIterScore01 :type "Float (double-precision)")))

(fn `FreezeAtCurrentPose`
  (set `self.bIsFrozen` true))

(fn `GetCurrentPose`
  (returns (OutPose :type "/Game/MovementComparison/Structs/S_GuidePoseFrame Structure") (bIsValid :type Boolean))
  (bind _bdataloaded (`self.bDataLoaded`))
  (return (make `/Game/MovementComparison/Structs/S_GuidePoseFrame` (`self.PlaybackTime`) _bdataloaded (`self.IK_Waist`) (`self.IK_LeftKnee`) (`self.IK_RightKnee`) (`self.IK_LeftFoot`) (`self.IK_RightFoot`) (`self.IK_LeftElbow`) (`self.IK_RightElbow`) (`self.IK_Head`) (`self.IK_LeftHand`) (`self.IK_RightHand`)) _bdataloaded))

(fn `GetInterpolatedSnapshot`
  (returns (OutSnapshot :type "/Game/Data/Recorder/Struct/S_TrackerSnapshot Structure") (bValid :type Boolean))
  (bind _teacherposes (`self.TeacherPoses`))
  (bind _localindex (`self.LocalIndex`))
  (bind _returnvalue (`KismetArrayLibrary.Array_Length` _teacherposes))
  (bind (_timestamp _bvalid _ik_waist _ik_leftknee _ik_rightknee _ik_leftfoot _ik_rightfoot _ik_leftelbow _ik_rightelbow _ik_head _ik_lefthand _ik_righthand) (break `/Game/MovementComparison/Structs/S_GuidePoseFrame` (`|GetArrayItem` _teacherposes)))
  (bind (_timestamp_2 _bvalid_2 _ik_waist_2 _ik_leftknee_2 _ik_rightknee_2 _ik_leftfoot_2 _ik_rightfoot_2 _ik_leftelbow_2 _ik_rightelbow_2 _ik_head_2 _ik_lefthand_2 _ik_righthand_2) (break `/Game/MovementComparison/Structs/S_GuidePoseFrame` (`|GetArrayItem` _teacherposes _localindex)))
  (bind (_timestamp_3 _bvalid_3 _ik_waist_3 _ik_leftknee_3 _ik_rightknee_3 _ik_leftfoot_3 _ik_rightfoot_3 _ik_leftelbow_3 _ik_rightelbow_3 _ik_head_3 _ik_lefthand_3 _ik_righthand_3) (break `/Game/MovementComparison/Structs/S_GuidePoseFrame` (`|GetArrayItem` _teacherposes (+ _localindex 1))))
  (bind _returnvalue_2 (`KismetMathLibrary.FClamp` (/ (- 0.0 _timestamp_2) (`KismetMathLibrary.FMax` (- _timestamp_3 _timestamp_2) 0.0001))))
  (if (== _returnvalue 0)
    _
    (elif (== _returnvalue 1)
      (return (make `/Game/Data/Recorder/Struct/S_TrackerSnapshot` _timestamp _ik_waist _ik_leftknee _ik_rightknee _ik_leftfoot _ik_rightfoot _ik_leftelbow _ik_rightelbow _ik_head _ik_lefthand _ik_righthand) true)
      (else
        (`|ExecutionSequence`
          (:`then_0`
            (set `self.LocalFound` false)
            (set `self.LocalIndex` 0)
            (for _index (range (+ (- _returnvalue 2) 1))
              (if (not (`self.LocalFound`))
                (if (and (<= (`.Timestamp_3_EB10FE0A4F83D665D9644FAFBD4AD520` (break `/Game/MovementComparison/Structs/S_GuidePoseFrame` (`|GetArrayItem` _teacherposes _index))) 0.0) (>= (`.Timestamp_3_EB10FE0A4F83D665D9644FAFBD4AD520` (break `/Game/MovementComparison/Structs/S_GuidePoseFrame` (`|GetArrayItem` _teacherposes (+ _index 1)))) 0.0))
                  (set `self.LocalFound` true)
                  (set `self.LocalFound` true)
                  (set `self.LocalIndex` _index))))
            (if (`self.LocalFound`)
              _
              (elif (< 0.0 (`.Timestamp_3_EB10FE0A4F83D665D9644FAFBD4AD520` (break `/Game/MovementComparison/Structs/S_GuidePoseFrame` (`|GetArrayItem` _teacherposes))))
                (set `self.LocalIndex` 0)
                (else
                  (set `self.LocalIndex` (- _returnvalue 2))))))
          (:`then_1`
            (return (make `/Game/Data/Recorder/Struct/S_TrackerSnapshot` (`KismetMathLibrary.Lerp` _timestamp_2 _timestamp_3 _returnvalue_2) (`KismetMathLibrary.TLerp` _ik_waist_2 _ik_waist_3 _returnvalue_2) (`KismetMathLibrary.TLerp` _ik_leftknee_2 _ik_leftknee_3 _returnvalue_2) (`KismetMathLibrary.TLerp` _ik_rightknee_2 _ik_rightknee_3 _returnvalue_2) (`KismetMathLibrary.TLerp` _ik_leftfoot_2 _ik_leftfoot_3 _returnvalue_2) (`KismetMathLibrary.TLerp` _ik_rightfoot_2 _ik_rightfoot_3 _returnvalue_2) (`KismetMathLibrary.TLerp` _ik_leftelbow_2 _ik_leftelbow_3 _returnvalue_2) (`KismetMathLibrary.TLerp` _ik_rightelbow_2 _ik_rightelbow_3 _returnvalue_2) (`KismetMathLibrary.TLerp` _ik_head_2 _ik_head_3 _returnvalue_2) (`KismetMathLibrary.TLerp` _ik_lefthand_2 _ik_lefthand_3 _returnvalue_2) (`KismetMathLibrary.TLerp` _ik_righthand_2 _ik_righthand_3 _returnvalue_2)) true)))))))

(fn `IsPoseFrozen`
  (returns (bFrozen :type Boolean))
  (return false))

(fn `LoadMovementFromCache`
  (params (MovementInfo :type "/Game/MovementComparison/Structs/S_MovementInfo Structure") (CacheRef1 :type "/Game/MovementComparison/Blueprints/BP_MovementCache Object Reference"))
  (returns (bSuccess :type Boolean) (ErrorMsg :type String))
  (bind (_movementname _category _saveslotname) (break `/Game/MovementComparison/Structs/S_MovementInfo` MovementInfo))
  (bind _proceduraltable (`self.ProceduralTable`))
  (bind _teacherposes (`self.TeacherPoses`))
  (if (`KismetSystemLibrary.IsValid` _proceduraltable)
    (bind _returnvalue (`|GetDataTableRow` _proceduraltable (`KismetStringLibrary.Conv_StringToName` (`.SaveSlotName_9_13EF4A5247E2757E95A2CD801B9F9F30` (break `/Game/MovementComparison/Structs/S_MovementInfo` MovementInfo))))
      (:`then`
        (`KismetArrayLibrary.Array_Clear` (`self.TeacherPoses`))
        (for _array_element (`.Keyframes_2_E5153A814C08EBE4F8D3398A7C5E46C8` (break `/Game/MovementComparison/Structs/S_ProceduralTechnique` _returnvalue))
          (`KismetArrayLibrary.Array_Add` (`self.TeacherPoses`) _array_element))
        (set `self.CurrentTeacherIndex` 0)
        (set `self.CurrentMovementInfo` MovementInfo)
        (set `self.bDataLoaded` true)
        (set `self.bHasError` false)
        (return true ""))
      (:`RowNotFound`
        _)))
  (`/Engine/EditorBlueprintResources/StandardMacros.IsValid` CacheRef1
    (:`Is Valid`
      (bind (_bsuccess _outsnapshots) (`/Game/MovementComparison/Blueprints/BP_MovementCache.GetSnapshots` CacheRef1 (`KismetStringLibrary.Conv_StringToName` _saveslotname)))
      (if (and _bsuccess (> (`KismetArrayLibrary.Array_Length` _outsnapshots) 0))
        (`KismetArrayLibrary.Array_Clear` _teacherposes)
        (for _array_element_2 _outsnapshots
          (bind (_timestamp _ik_waist _ik_leftknee _ik_rightknee _ik_leftfoot _ik_rightfoot _ik_leftelbow _ik_rightelbow _ik_head _ik_lefthand _ik_righthand) (break `/Game/Data/Recorder/Struct/S_TrackerSnapshot` _array_element_2))
          (`KismetArrayLibrary.Array_Add` _teacherposes (make `/Game/MovementComparison/Structs/S_GuidePoseFrame` _timestamp true _ik_waist _ik_leftknee _ik_rightknee _ik_leftfoot _ik_rightfoot _ik_leftelbow _ik_rightelbow _ik_head _ik_lefthand _ik_righthand)))
        (set `self.CurrentTeacherIndex` 0)
        (set `self.CurrentMovementInfo` MovementInfo)
        (set `self.bDataLoaded` true)
        (set `self.bHasError` false)
        (set `self.LastErrorMessage` "")
        (set `self.LastErrorMessage` "")
        (return true "")
        (else
          (set `self.bDataLoaded` false)
          (return false (`KismetStringLibrary.Concat_StrStr` "LoadMovementFromCache: no snapshots for slot " _saveslotname)))))
    (:`Is Not Valid`
      (set `self.bDataLoaded` false)
      (return false "LoadMovementFromCache: CacheRef invalid"))))

(fn `PlayPhase`
  (returns (bSuccess :type Boolean))
  (return false))

(fn `ResetGuide`)

(fn `StopPlayback`
  (set `self.bIsPlaying` false))

(fn `UserConstructionScript`)