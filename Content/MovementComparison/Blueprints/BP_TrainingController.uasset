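; Training controller that runs the movement-training menu flow, from category and movement selection to demonstration and results.
; It reads movements from a data table, hands itself and data to BP_TrainingStation panel widgets, and spawns a guide facing the player.
; The guide plays a slowed animation, and fixed delays, rather than animation completion, lead to the results panel.
; State changes are logged and broadcast to itself through BPI_TrainingEvents, with failures routed through RaiseError.
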(event `self.ReceiveBeginPlay`
  (`KismetSystemLibrary.Delay` 0.2)
  (`self.InitializeTraining`))

(event `StartDemonstration`
  (bind _returnvalue (`self.GetComponentByClass` (`self.GuideRef`) "/Script/Engine.SkeletalMeshComponent"))
  (`self.SetTrainingState` "NewEnumerator9")
  (`SkeletalMeshComponent.PlayAnimation` _returnvalue (`.DemoAnimSequence_14_279136A34B5F78617D9A4E82ED8E98DC` (break `/Game/MovementComparison/Structs/S_MovementInfo` (`self.CurrentMovementInfo`))) false)
  (`SkeletalMeshComponent.SetPlayRate` _returnvalue 0.3)
  (`KismetSystemLibrary.Delay` 16.0)
  (`KismetSystemLibrary.PrintString` "Demo Terminada - Countdown 3s")
  (`KismetSystemLibrary.Delay` 3.0)
  (`self.ShowResultsPanel`))

(event `StartSalvavidas`
  (`KismetSystemLibrary.Delay` 30.0)
  (if (`|EnumEquality` (`self.TrainingState`) (enumliteral `/Game/MovementComparison/Enums/E_TrainingState` "NewEnumerator4"))
    (`self.SetTrainingState` (enumliteral `/Game/MovementComparison/Enums/E_TrainingState` "NewEnumerator8"))
    (`self.RaiseError` "SALVAVIDAS timeout - evaluación superó límite de tiempo")))

(event `/Game/MovementComparison/Interfaces/BPI_TrainingEvents.OnCategorySelected`
  (params (Category :type "/Game/MovementComparison/Enums/E_MovementCategory Enum" :default "NewEnumerator0"))
  (set `self.CurrentCategory` Category)
  (`self.ShowMovementList`))

(event `/Game/MovementComparison/Interfaces/BPI_TrainingEvents.OnBackToMenu`
  (`self.SafeDestroyGuide`)
  (`self.ShowMainMenu`))

(event `/Game/MovementComparison/Interfaces/BPI_TrainingEvents.OnMovementSelected`
  (params (MovementRowName :type Name))
  (`KismetSystemLibrary.PrintString` (`KismetStringLibrary.Concat_StrStr` "[Trainer] OnMovementSelected: " (`KismetStringLibrary.Conv_NameToString` MovementRowName)) true true (struct :`G` 1.0 :`A` 1.0) 5.0)
  (bind (_bfound _outinfo) (`self.SafeGetMovementInfo` MovementRowName))
  (if _bfound
    (set `self.CurrentMovementRowName` MovementRowName)
    (set `self.CurrentMovementInfo` _outinfo)
    (`self.BeginMovementFlow`)
    (else
      (`self.RaiseError` "Movement not found in table"))))

(event `/Game/MovementComparison/Interfaces/BPI_TrainingEvents.OnStartPressed`
  (`self.StartDemonstration`))

(fn `BeginMovementFlow`
  (bind _bsuccess (`self.SafeSpawnGuide`))
  (if (not _bsuccess)
    (`self.RaiseError` "SafeSpawnGuide failed")
    (else
      (`KismetArrayLibrary.Array_Clear` (`self.OutRowNames`))
      (`self.ShowStartPanel`))))

(fn `EnsureWidgetsCreated`
  (returns (bSuccess :type Boolean))
  (return true))

(fn `GetMovementsForCategory`
  (params (Category :type "/Game/MovementComparison/Enums/E_MovementCategory Enum" :default "NewEnumerator0"))
  (returns (OutRowNames :type "Array of Name") (OutInfos :type "Array of /Game/MovementComparison/Structs/S_MovementInfo Structure"))
  (bind _movementstable (`self.MovementsTable`))
  (bind _outrownames (`self.OutRowNames`))
  (bind _localinfos (`self.LocalInfos`))
  (`KismetArrayLibrary.Array_Clear` _outrownames)
  (`KismetArrayLibrary.Array_Clear` _localinfos)
  (`/Engine/EditorBlueprintResources/StandardMacros.IsValid` _movementstable
    (:`Is Valid`
      (bind _outrownames_2 (`DataTableFunctionLibrary.GetDataTableRowNames` _movementstable))
      (for _array_element _outrownames_2
        (bind _returnvalue (`|GetDataTableRow` _movementstable _array_element)
          (:`then`
            (if (or (`|EnumEquality` Category (enumliteral `/Game/MovementComparison/Enums/E_MovementCategory` "NewEnumerator0")) (`|EnumEquality` (`.Category_8_EA9E353C4405097407275B891F40BB71` (break `/Game/MovementComparison/Structs/S_MovementInfo` _returnvalue)) Category))
              (`KismetArrayLibrary.Array_AddUnique` _outrownames _array_element)
              (`KismetArrayLibrary.Array_Add` _localinfos _returnvalue)))))
      (return _outrownames _localinfos))
    (:`Is Not Valid`
      (return _outrownames _localinfos))))

(fn `HideAllWidgets`
  (bind _outactors (`GameplayStatics.GetAllActorsOfClass` "/Game/MovementComparison/Blueprints/BP_TrainingStation.BP_TrainingStation_C"))
  (if (> (`KismetArrayLibrary.Array_Length` _outactors) 0)
    (bind _asbp_training_station (cast `/Game/MovementComparison/Blueprints/BP_TrainingStation` (`|GetArrayItem` _outactors)))
    (`/Game/MovementComparison/Blueprints/BP_TrainingStation.HideAllPanels` _asbp_training_station)))

(fn `InitializeTraining`
  (returns (bSuccess :type Boolean))
  (bind (_outpawn _bfound) (`self.SafeFindUserPawn` self))
  (if (not _bfound)
    (`self.RaiseError` self "User pawn not found")
    (return false)
    (else
      (bind _bsuccess (`self.EnsureWidgetsCreated` self))
      (if (not _bsuccess)
        (return false)
        (else
          (`self.SetTrainingState` self (enumliteral `/Game/MovementComparison/Enums/E_TrainingState` "NewEnumerator1"))
          (`self.ShowMainMenu` self)
          (return true))))))

(fn `RaiseError`
  (params (Msg :type String))
  (set `self.bHasError` true)
  (set `self.LastErrorMessage` Msg)
  (`KismetSystemLibrary.PrintString` (`KismetStringLibrary.Concat_StrStr` "[Trainer] " Msg) true true (struct :`R` 1.0 :`A` 1.0))
  (`self.SetTrainingState` (enumliteral `/Game/MovementComparison/Enums/E_TrainingState` "NewEnumerator8")))

(fn `SafeDestroyGuide`
  (bind _guideref (`self.GuideRef`))
  (`/Engine/EditorBlueprintResources/StandardMacros.IsValid` _guideref
    (:`Is Valid`
      (`self.K2_DestroyActor` _guideref)
      (set `self.GuideRef` null))))

(fn `SafeFindCache`
  (returns (bFound :type Boolean) (OutCache1 :type "/Game/MovementComparison/Blueprints/BP_MovementCache Object Reference"))
  (bind _outactors (`GameplayStatics.GetAllActorsOfClass` self "/Game/MovementComparison/Blueprints/BP_MovementCache.BP_MovementCache_C"))
  (if (> (`KismetArrayLibrary.Array_Length` _outactors) 0)
    (bind _output (`|GetArrayItem` _outactors))
    (set `self.CacheRef` _output)
    (return true _output)
    (else
      (return false null))))

(fn `SafeFindUserPawn`
  (returns (OutPawn :type "Actor Object Reference") (bFound :type Boolean))
  (bind _returnvalue (`GameplayStatics.GetPlayerPawn` self))
  (`/Engine/EditorBlueprintResources/StandardMacros.IsValid` _returnvalue
    (:`Is Valid`
      (set `self.UserRef` _returnvalue)
      (return _returnvalue true))
    (:`Is Not Valid`
      (return null false))))

(fn `SafeGetMovementInfo`
  (params (RowName :type Name))
  (returns (bFound :type Boolean) (OutInfo :type "/Game/MovementComparison/Structs/S_MovementInfo Structure"))
  (bind _returnvalue (`|GetDataTableRow` (`self.MovementsTable`) RowName)
    (:`then`
      (return true _returnvalue))
    (:`RowNotFound`
      (return false (make `/Game/MovementComparison/Structs/S_MovementInfo` :`DemoAnimSequence` null)))))

(fn `SafeSpawnGuide`
  (returns (bSuccess :type Boolean))
  (bind _guideref (`self.GuideRef`))
  (bind _userref (`self.UserRef`))
  (bind _returnvalue (`self.K2_GetActorLocation` _userref))
  (bind _returnvalue_2 (`KismetMathLibrary.MakeVector` (.x (+ _returnvalue (+ (* (`self.GetActorForwardVector` _userref) 150.0) (* (`self.GetActorRightVector` _userref) 100.0)))) (.y (+ _returnvalue (+ (* (`self.GetActorForwardVector` _userref) 150.0) (* (`self.GetActorRightVector` _userref) 100.0)))) (+ (.z _returnvalue) 40.0)))
  (`|ExecutionSequence`
    (:`then_0`
      (`/Engine/EditorBlueprintResources/StandardMacros.IsValid` _guideref
        (:`Is Valid`
          (`self.K2_DestroyActor` _guideref)
          (set `self.GuideRef` null))))
    (:`then_1`
      (bind _returnvalue_3 (`|SpawnActorFromClass` (`self.GuideClass`) (`KismetMathLibrary.MakeTransform` _returnvalue_2 (`KismetMathLibrary.MakeRotator` 0.0 0.0 (.yaw (`KismetMathLibrary.FindLookAtRotation` _returnvalue_2 _returnvalue))) (`KismetMathLibrary.MakeVector` 1.0 1.0 1.0)) "AlwaysSpawn" "SelectDefaultAtRuntime" self null))
      (`/Engine/EditorBlueprintResources/StandardMacros.IsValid` _returnvalue_3
        (:`Is Valid`
          (bind _asbp_guide_character (cast `/Game/MovementComparison/Blueprints/BP_GuideCharacter` _returnvalue_3)
            (:`then`
              (set `self.GuideRef` _asbp_guide_character)
              (return true))
            (:`CastFailed`
              (return false))))
        (:`Is Not Valid`
          (return false))))))

(fn `SetTrainingState`
  (params (NewState :type "/Game/MovementComparison/Enums/E_TrainingState Enum" :default "NewEnumerator0"))
  (`|ExecutionSequence`
    (:`then_0`
      (if (`KismetSystemLibrary.DoesImplementInterface` self "/Game/MovementComparison/Interfaces/BPI_TrainingEvents.BPI_TrainingEvents_C")
        (message `/Game/MovementComparison/Interfaces/BPI_TrainingEvents.OnTrainingStateChanged` self NewState)))
    (:`then_1`
      (`KismetSystemLibrary.PrintString` (`KismetStringLibrary.Concat_StrStr` "[Trainer] State -> " (`|GetEnumeratorNameAsString` NewState))))))

(fn `ShowMainMenu`
  (bind _outactors (`GameplayStatics.GetAllActorsOfClass` "/Game/MovementComparison/Blueprints/BP_TrainingStation.BP_TrainingStation_C"))
  (if (> (`KismetArrayLibrary.Array_Length` _outactors) 0)
    (bind _asbp_training_station (cast `/Game/MovementComparison/Blueprints/BP_TrainingStation` (`|GetArrayItem` _outactors)))
    (`/Game/MovementComparison/Blueprints/BP_TrainingStation.ShowOnlyPanel` _asbp_training_station "MainMenu")
    (bind _widget (`/Game/MovementComparison/Blueprints/BP_TrainingStation.GetWidgetForPanel` _asbp_training_station "MainMenu"))
    (bind _aswbp_main_menu (cast `/Game/MovementComparison/Widgets/WBP_MainMenu` _widget))
    (set `self.MainMenuRef` _aswbp_main_menu)
    (set `/Game/MovementComparison/Widgets/WBP_MainMenu.ControllerRef` self _aswbp_main_menu)))

(fn `ShowMovementList`
  (bind _outactors (`GameplayStatics.GetAllActorsOfClass` "/Game/MovementComparison/Blueprints/BP_TrainingStation.BP_TrainingStation_C"))
  (if (> (`KismetArrayLibrary.Array_Length` _outactors) 0)
    (bind _asbp_training_station (cast `/Game/MovementComparison/Blueprints/BP_TrainingStation` (`|GetArrayItem` _outactors)))
    (`/Game/MovementComparison/Blueprints/BP_TrainingStation.ShowOnlyPanel` _asbp_training_station "MovementList")
    (bind _widget (`/Game/MovementComparison/Blueprints/BP_TrainingStation.GetWidgetForPanel` _asbp_training_station "MovementList"))
    (bind _aswbp_movement_list (cast `/Game/MovementComparison/Widgets/WBP_MovementList` _widget))
    (set `/Game/MovementComparison/Widgets/WBP_MovementList.ControllerRef` self _aswbp_movement_list)
    (set `self.MovementListRef` _aswbp_movement_list)
    (`/Game/MovementComparison/Widgets/WBP_MovementList.PopulateList` _aswbp_movement_list (`self.CurrentCategory`))))

(fn `ShowResultsPanel`
  (bind _outactors (`GameplayStatics.GetAllActorsOfClass` "/Game/MovementComparison/Blueprints/BP_TrainingStation.BP_TrainingStation_C"))
  (if (> (`KismetArrayLibrary.Array_Length` _outactors) 0)
    (bind _asbp_training_station (cast `/Game/MovementComparison/Blueprints/BP_TrainingStation` (`|GetArrayItem` _outactors)))
    (`/Game/MovementComparison/Blueprints/BP_TrainingStation.ShowOnlyPanel` _asbp_training_station "Results")
    (bind _widget (`/Game/MovementComparison/Blueprints/BP_TrainingStation.GetWidgetForPanel` _asbp_training_station "Results"))
    (bind _aswbp_results_panel (cast `/Game/MovementComparison/Widgets/WBP_ResultsPanel` _widget))
    (set `/Game/MovementComparison/Widgets/WBP_ResultsPanel.ControllerRef` self _aswbp_results_panel)))

(fn `ShowStartPanel`
  (bind _outactors (`GameplayStatics.GetAllActorsOfClass` "/Game/MovementComparison/Blueprints/BP_TrainingStation.BP_TrainingStation_C"))
  (if (> (`KismetArrayLibrary.Array_Length` _outactors) 0)
    (bind _asbp_training_station (cast `/Game/MovementComparison/Blueprints/BP_TrainingStation` (`|GetArrayItem` _outactors)))
    (`/Game/MovementComparison/Blueprints/BP_TrainingStation.ShowOnlyPanel` _asbp_training_station "StartPanel")
    (bind _widget (`/Game/MovementComparison/Blueprints/BP_TrainingStation.GetWidgetForPanel` _asbp_training_station "StartPanel"))
    (bind _aswbp_start_panel (cast `/Game/MovementComparison/Widgets/WBP_StartPanel` _widget))
    (set `/Game/MovementComparison/Widgets/WBP_StartPanel.ControllerRef` self _aswbp_start_panel)
    (set `self.StartPanelRef` _aswbp_start_panel)
    (set `/Game/MovementComparison/Widgets/WBP_StartPanel.MovementInfo` (`self.CurrentMovementInfo`) _aswbp_start_panel)))

(fn `ShowTrainingHUD`
  (bind _outactors (`GameplayStatics.GetAllActorsOfClass` "/Game/MovementComparison/Blueprints/BP_TrainingStation.BP_TrainingStation_C"))
  (if (> (`KismetArrayLibrary.Array_Length` _outactors) 0)
    (bind _asbp_training_station (cast `/Game/MovementComparison/Blueprints/BP_TrainingStation` (`|GetArrayItem` _outactors)))
    (`/Game/MovementComparison/Blueprints/BP_TrainingStation.ShowOnlyPanel` _asbp_training_station "HUD")
    (bind _widget (`/Game/MovementComparison/Blueprints/BP_TrainingStation.GetWidgetForPanel` _asbp_training_station "HUD"))
    (bind _aswbp_training_hud (cast `/Game/MovementComparison/Widgets/WBP_TrainingHUD` _widget))
    (set `self.TrainingHUDRef` _aswbp_training_hud)
    (`/Game/MovementComparison/Widgets/WBP_TrainingHUD.BuildIndicators` _aswbp_training_hud)))

(fn `UserConstructionScript`)