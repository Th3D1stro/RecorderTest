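; VR player character that turns headset, hand, waist and foot tracking into mesh-space IK transforms for a full-body avatar.
; A calibration input stores each tracker's inverse rotation as an offset and derives a height scale factor.
; Tick applies the offsets, smoothing waist and feet with last-valid fallback on tracking loss; knee, elbow and pole-vector functions are empty stubs.
; It also drives left/right widget-interaction menu clicks and sets up VR tracking on BeginPlay.
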(event `self.ReceiveActorBeginOverlap`
  (params (OtherActor :type "Actor Object Reference")))

(event `EnhancedInput|/Game/XRFramework/Input/Actions/IA_Menu_Interact_Left_Pressed`
  (params (ActionValue :type Boolean) (ElapsedSeconds :type "Float (double-precision)") (TriggeredSeconds :type "Float (double-precision)") (InputAction :type "InputAction Object Reference" :default "/Game/XRFramework/Input/Actions/IA_Menu_Interact_Left_Pressed.IA_Menu_Interact_Left_Pressed"))
  (:`Started`
    (`WidgetInteractionComponent.PressPointerKey` (`self.WidgetInteraction_Left`) "LeftMouseButton")
    (`KismetSystemLibrary.PrintString` "Left trigger Started"))
  (:`Canceled`
    (`WidgetInteractionComponent.ReleasePointerKey` (`self.WidgetInteraction_Left`) "LeftMouseButton" :!label _label))
  (:`Completed`
    (goto _label)))

(event `EnhancedInput|/Game/XRFramework/Input/Actions/IA_CalibratePlayer`
  (params (ActionValue :type Boolean) (ElapsedSeconds :type "Float (double-precision)") (TriggeredSeconds :type "Float (double-precision)") (InputAction :type "InputAction Object Reference" :default "/Game/XRFramework/Input/Actions/IA_CalibratePlayer.IA_CalibratePlayer"))
  (:`Started`
    (`self.CalibrateFullBody`)))

(event `self.ReceiveTick`
  (params (DeltaSeconds :type "Float (single-precision)"))
  (`|ExecutionSequence`
    (:`then_0`
      (`self.UpdateWaistTracker`))
    (:`then_1`)
    (:`then_2`)
    (:`then_3`
      (`self.UpdateLeftFootTracker`))
    (:`then_4`
      (`self.UpdateRightFootTracker`))
    (:`then_5`)
    (:`then_6`)
    (:`then_7`
      (`self.UpdateHeadTracker`))
    (:`then_8`
      (`self.UpdateLeftHandTracker`))
    (:`then_9`
      (`self.UpdateRightHandTracker`))))

(event `EnhancedInput|/Game/XRFramework/Input/Actions/IA_Menu_Interact_Right_Pressed`
  (params (ActionValue :type Boolean) (ElapsedSeconds :type "Float (double-precision)") (TriggeredSeconds :type "Float (double-precision)") (InputAction :type "InputAction Object Reference" :default "/Game/XRFramework/Input/Actions/IA_Menu_Interact_Right_Pressed.IA_Menu_Interact_Right_Pressed"))
  (:`Started`
    (`WidgetInteractionComponent.PressPointerKey` (`self.WidgetInteraction_Right`) "LeftMouseButton")
    (`KismetSystemLibrary.PrintString` "Right trigger Started"))
  (:`Canceled`
    (`WidgetInteractionComponent.ReleasePointerKey` (`self.WidgetInteraction_Right`) "LeftMouseButton" :!label _label_2))
  (:`Completed`
    (goto _label_2)))

(event `self.ReceiveBeginPlay`
  (`self.BeginFunction`)
  (`EnhancedInputSubsystemInterface.AddMappingContext` (pcsubsystem `EnhancedInputLocalPlayerSubsystem` (`GameplayStatics.GetPlayerController` 0)) "/Game/XRFramework/Input/IMC_Menu.IMC_Menu" 1 (struct))
  (`KismetSystemLibrary.PrintString` "VR_CharacterBP possessed + IMC_Menu added"))

(fn `BeginFunction`
  (set `self.CharacterMesh0` (`self.Mesh`))
  (if (`HeadMountedDisplayFunctionLibrary.IsHeadMountedDisplayEnabled`)
    (`|ExecutionSequence`
      (:`then_0`
        (`HeadMountedDisplayFunctionLibrary.SetTrackingOrigin` "LocalFloor")
        (`KismetSystemLibrary.ExecuteConsoleCommand` "xr.SecondaryScreenPercentage.HMDRenderTarget 100" null)
        (`EnhancedInputSubsystemInterface.AddMappingContext` (pcsubsystem `EnhancedInputLocalPlayerSubsystem` (`GameplayStatics.GetPlayerController` 0)) "/Game/Players/Player_Level2/Calibration.Calibration" 0 (struct)))
      (:`then_1`
        (`XRLoadingScreenFunctionLibrary.HideLoadingScreen`) ; See WidgetMenu for loading screen logic
      ))))

(fn `CalibrateFullBody`
  (bind _head (`self.Head`))
  (bind _returnvalue (`KismetMathLibrary.FClamp` (`KismetMathLibrary.SafeDivide` (- (.z (`SceneComponent.K2_GetComponentLocation` _head)) (.z (`SceneComponent.K2_GetComponentLocation` (`self.VROrigin`)))) 183.0) 0.5 2.0))
  (set `self.FactorEscala` _returnvalue)
  (`self.CalibrationHead` (`SceneComponent.K2_GetComponentToWorld` _head))
  (`self.CalibrationWaist` (`SceneComponent.K2_GetComponentToWorld` (`self.Waist`)))
  (`self.CalibrationLeftHand` (`SceneComponent.K2_GetComponentToWorld` (`self.LeftHand`)))
  (`self.CalibrationRightHand` (`SceneComponent.K2_GetComponentToWorld` (`self.RightHand`)))
  (`self.CalibrationLeftFoot` (`SceneComponent.K2_GetComponentToWorld` (`self.LeftFoot`)))
  (`self.CalibrationRightFoot` (`SceneComponent.K2_GetComponentToWorld` (`self.RightFoot`)))
  (set `self.bAllTrackersCalibrated` true)
  (`KismetSystemLibrary.PrintString` (`KismetStringLibrary.Concat_StrStr` (`KismetStringLibrary.Concat_StrStr` "[CalibrateFullBody] FactorEscala=" (`KismetStringLibrary.Conv_DoubleToString` _returnvalue)) " bAllTrackersCalibrated=true")))

(fn `CalibrationHead`
  (params (CalibrateTransform_Head :type "Transform Structure"))
  (bind _returnvalue (`KismetMathLibrary.ComposeTransforms` (`SceneComponent.K2_GetComponentToWorld` (`self.Head`)) (`KismetMathLibrary.InvertTransform` (`SceneComponent.K2_GetComponentToWorld` (`self.CharacterMesh0`)))))
  (set `self.CalibRef_Head` _returnvalue)
  (set `self.RotationOffset_Head` (`KismetMathLibrary.Quat_Rotator` (`KismetMathLibrary.Quat_Inversed` (`KismetMathLibrary.Conv_RotatorToQuaternion` (.rotation _returnvalue))))))

(fn `CalibrationLeftElbow`
  (params (CalibrateTransform_LeftElbow :type "Transform Structure")))

(fn `CalibrationLeftFoot`
  (params (CalibrateTransform_LeftFoot :type "Transform Structure"))
  (bind _returnvalue (`KismetMathLibrary.ComposeTransforms` (`SceneComponent.K2_GetComponentToWorld` (`self.LeftFoot`)) (`KismetMathLibrary.InvertTransform` (`SceneComponent.K2_GetComponentToWorld` (`self.CharacterMesh0`)))))
  (set `self.LastValidTransform_LeftFoot` CalibrateTransform_LeftFoot)
  (set `self.CalibRef_LeftFoot` _returnvalue)
  (set `self.RotationOffset_LeftFoot` (`KismetMathLibrary.Quat_Rotator` (`KismetMathLibrary.Quat_Inversed` (`KismetMathLibrary.Conv_RotatorToQuaternion` (.rotation _returnvalue)))))
  (set `self.bIsCalibrated_LeftFoot` true))

(fn `CalibrationLeftHand`
  (params (CalibrateTransform_LeftHand :type "Transform Structure"))
  (bind _returnvalue (`KismetMathLibrary.ComposeTransforms` (`SceneComponent.K2_GetComponentToWorld` (`self.LeftHand`)) (`KismetMathLibrary.InvertTransform` (`SceneComponent.K2_GetComponentToWorld` (`self.CharacterMesh0`)))))
  (set `self.CalibRef_LeftHand` _returnvalue)
  (set `self.RotationOffset_LeftHand` (`KismetMathLibrary.Quat_Rotator` (`KismetMathLibrary.Quat_Inversed` (`KismetMathLibrary.Conv_RotatorToQuaternion` (.rotation _returnvalue))))))

(fn `CalibrationLeftKnee`
  (params (CalibrateTransform_LeftKnee :type "Transform Structure")))

(fn `CalibrationRightElbow`
  (params (CalibrateTransform_RightElbow :type "Transform Structure")))

(fn `CalibrationRightFoot`
  (params (CalibrateTransform_RightFoot :type "Transform Structure"))
  (bind _returnvalue (`KismetMathLibrary.ComposeTransforms` (`SceneComponent.K2_GetComponentToWorld` (`self.RightFoot`)) (`KismetMathLibrary.InvertTransform` (`SceneComponent.K2_GetComponentToWorld` (`self.CharacterMesh0`)))))
  (set `self.LastValidTransform_RightFoot` CalibrateTransform_RightFoot)
  (set `self.CalibRef_RightFoot` _returnvalue)
  (set `self.RotationOffset_RightFoot` (`KismetMathLibrary.Quat_Rotator` (`KismetMathLibrary.Quat_Inversed` (`KismetMathLibrary.Conv_RotatorToQuaternion` (.rotation _returnvalue)))))
  (set `self.bIsCalibrated_RightFoot` true))

(fn `CalibrationRightHand`
  (params (CalibrateTransform_RightHand :type "Transform Structure"))
  (bind _returnvalue (`KismetMathLibrary.ComposeTransforms` (`SceneComponent.K2_GetComponentToWorld` (`self.RightHand`)) (`KismetMathLibrary.InvertTransform` (`SceneComponent.K2_GetComponentToWorld` (`self.CharacterMesh0`)))))
  (set `self.CalibRef_RightHand` _returnvalue)
  (set `self.RotationOffset_RightHand` (`KismetMathLibrary.Quat_Rotator` (`KismetMathLibrary.Quat_Inversed` (`KismetMathLibrary.Conv_RotatorToQuaternion` (.rotation _returnvalue))))))

(fn `CalibrationRightKnee`
  (params (CalibrateTransform_RightKnee :type "Transform Structure")))

(fn `CalibrationWaist`
  (params (CalibrateTransform_Waist :type "Transform Structure"))
  (bind _returnvalue (`KismetMathLibrary.ComposeTransforms` (`SceneComponent.K2_GetComponentToWorld` (`self.Waist`)) (`KismetMathLibrary.InvertTransform` (`SceneComponent.K2_GetComponentToWorld` (`self.CharacterMesh0`)))))
  (set `self.LastValidTransform_Waist` CalibrateTransform_Waist)
  (set `self.CalibRef_Waist` _returnvalue)
  (set `self.RotationOffset_Waist` (`KismetMathLibrary.Quat_Rotator` (`KismetMathLibrary.Quat_Inversed` (`KismetMathLibrary.Conv_RotatorToQuaternion` (.rotation _returnvalue)))))
  (set `self.blsCalibrated_Waist` true))

(fn `ComputeAndApplyPoleVectors`)

(fn `DebugFunction`
  (params (DebugTransform :type "Transform Structure"))
  (bind _location (.location DebugTransform))
  (`KismetSystemLibrary.DrawDebugSphere` _location 5.0 12 (struct :`R` 1.0 :`G` 0.680213 :`A` 1.0))
  (`KismetSystemLibrary.PrintString` (`KismetStringLibrary.Conv_VectorToString` _location) false false)
  (`KismetSystemLibrary.PrintText` (`KismetTextLibrary.Conv_RotatorToText` (.rotation DebugTransform)) false false))

(fn `LogIKFunction`
  (params (LogTransform :type "Transform Structure") (TrackerName :type String))
  (`KismetSystemLibrary.PrintString` (`KismetStringLibrary.Concat_StrStr` (`KismetStringLibrary.Concat_StrStr` (`KismetStringLibrary.Concat_StrStr` (`KismetStringLibrary.Concat_StrStr` TrackerName " Loc:") (`KismetStringLibrary.Conv_VectorToString` (.location LogTransform))) " Rot:") (`KismetStringLibrary.Conv_RotatorToString` (.rotation LogTransform))) false false (struct :`G` 0.66 :`B` 1.0 :`A` 1.0) 0.0))

(fn `UpdateHeadTracker`
  (if (`HeadMountedDisplayFunctionLibrary.IsHeadMountedDisplayEnabled`)
    (set `self.IK_Head` (`KismetMathLibrary.MakeTransform` (.location (`KismetMathLibrary.ComposeTransforms` (`SceneComponent.K2_GetComponentToWorld` (`self.Head`)) (`KismetMathLibrary.InvertTransform` (`SceneComponent.K2_GetComponentToWorld` (`self.CharacterMesh0`))))) (`KismetMathLibrary.ComposeRotators` (`self.RotationOffset_Head`) (.rotation (`KismetMathLibrary.ComposeTransforms` (`SceneComponent.K2_GetComponentToWorld` (`self.Head`)) (`KismetMathLibrary.InvertTransform` (`SceneComponent.K2_GetComponentToWorld` (`self.CharacterMesh0`)))))) (.scale (`KismetMathLibrary.ComposeTransforms` (`SceneComponent.K2_GetComponentToWorld` (`self.Head`)) (`KismetMathLibrary.InvertTransform` (`SceneComponent.K2_GetComponentToWorld` (`self.CharacterMesh0`)))))))
    (`self.LogIKFunction` (`self.IK_Head`) "IK_Head")))

(fn `UpdateLeftFootTracker`
  (bind _leftfoot (`self.LeftFoot`))
  (bind _returnvalue (`MotionControllerComponent.IsTracked` _leftfoot))
  (if (`self.bIsCalibrated_LeftFoot`)
    (`|ExecutionSequence`
      (:`then_0`
        (if _returnvalue
          (set `self.LastValidTransform_LeftFoot` (`SceneComponent.K2_GetComponentToWorld` _leftfoot))))
      (:`then_1`
        (set `self.IK_LeftFoot` (`KismetMathLibrary.TLerp` (`KismetMathLibrary.MakeTransform` (.location (`KismetMathLibrary.ComposeTransforms` (`KismetMathLibrary.SelectTransform` (`SceneComponent.K2_GetComponentToWorld` _leftfoot) (`self.LastValidTransform_LeftFoot`) _returnvalue) (`KismetMathLibrary.InvertTransform` (`SceneComponent.K2_GetComponentToWorld` (`self.CharacterMesh0`))))) (`KismetMathLibrary.ComposeRotators` (`self.RotationOffset_LeftFoot`) (.rotation (`KismetMathLibrary.ComposeTransforms` (`KismetMathLibrary.SelectTransform` (`SceneComponent.K2_GetComponentToWorld` _leftfoot) (`self.LastValidTransform_LeftFoot`) _returnvalue) (`KismetMathLibrary.InvertTransform` (`SceneComponent.K2_GetComponentToWorld` (`self.CharacterMesh0`)))))) (.scale (`KismetMathLibrary.ComposeTransforms` (`KismetMathLibrary.SelectTransform` (`SceneComponent.K2_GetComponentToWorld` _leftfoot) (`self.LastValidTransform_LeftFoot`) _returnvalue) (`KismetMathLibrary.InvertTransform` (`SceneComponent.K2_GetComponentToWorld` (`self.CharacterMesh0`)))))) (`self.IK_LeftFoot`) (`KismetMathLibrary.FClamp` (* (* (`self.FilterStrength_LeftFoot`) (`GameplayStatics.GetWorldDeltaSeconds`)) 60.0)))))
      (:`then_2`
        (`self.LogIKFunction` (`self.IK_LeftFoot`) "IK_LeftFoot")))))

(fn `UpdateLeftHandTracker`
  (bind _lefthand (`self.LeftHand`))
  (if (`MotionControllerComponent.IsTracked` _lefthand)
    (set `self.IK_LeftHand` (`KismetMathLibrary.MakeTransform` (.location (`KismetMathLibrary.ComposeTransforms` (`SceneComponent.K2_GetComponentToWorld` _lefthand) (`KismetMathLibrary.InvertTransform` (`SceneComponent.K2_GetComponentToWorld` (`self.CharacterMesh0`))))) (`KismetMathLibrary.ComposeRotators` (`self.RotationOffset_LeftHand`) (.rotation (`KismetMathLibrary.ComposeTransforms` (`SceneComponent.K2_GetComponentToWorld` _lefthand) (`KismetMathLibrary.InvertTransform` (`SceneComponent.K2_GetComponentToWorld` (`self.CharacterMesh0`)))))) (.scale (`KismetMathLibrary.ComposeTransforms` (`SceneComponent.K2_GetComponentToWorld` _lefthand) (`KismetMathLibrary.InvertTransform` (`SceneComponent.K2_GetComponentToWorld` (`self.CharacterMesh0`)))))))
    (`self.LogIKFunction` (`self.IK_LeftHand`) "IK_LeftHand")))

(fn `UpdateRightFootTracker`
  (bind _rightfoot (`self.RightFoot`))
  (bind _returnvalue (`MotionControllerComponent.IsTracked` _rightfoot))
  (bind _returnvalue_2 (`SceneComponent.K2_GetComponentToWorld` _rightfoot))
  (if (`self.bIsCalibrated_RightFoot`)
    (`|ExecutionSequence`
      (:`then_0`
        (if _returnvalue
          (set `self.LastValidTransform_RightFoot` _returnvalue_2)))
      (:`then_1`
        (set `self.IK_RightFoot` (`KismetMathLibrary.TLerp` (`KismetMathLibrary.MakeTransform` (.location (`KismetMathLibrary.ComposeTransforms` (`KismetMathLibrary.SelectTransform` _returnvalue_2 (`self.LastValidTransform_RightFoot`) _returnvalue) (`KismetMathLibrary.InvertTransform` (`SceneComponent.K2_GetComponentToWorld` (`self.CharacterMesh0`))))) (`KismetMathLibrary.ComposeRotators` (`self.RotationOffset_RightFoot`) (.rotation (`KismetMathLibrary.ComposeTransforms` (`KismetMathLibrary.SelectTransform` _returnvalue_2 (`self.LastValidTransform_RightFoot`) _returnvalue) (`KismetMathLibrary.InvertTransform` (`SceneComponent.K2_GetComponentToWorld` (`self.CharacterMesh0`)))))) (.scale (`KismetMathLibrary.ComposeTransforms` (`KismetMathLibrary.SelectTransform` _returnvalue_2 (`self.LastValidTransform_RightFoot`) _returnvalue) (`KismetMathLibrary.InvertTransform` (`SceneComponent.K2_GetComponentToWorld` (`self.CharacterMesh0`)))))) (`self.IK_RightFoot`) (`KismetMathLibrary.FClamp` (* (* (`self.FilterStrength_RightFoot`) (`GameplayStatics.GetWorldDeltaSeconds`)) 60.0)))))
      (:`then_2`
        (`self.LogIKFunction` (`self.IK_RightFoot`) "IK_RightFoot")))))

(fn `UpdateRightHandTracker`
  (bind _righthand (`self.RightHand`))
  (if (`MotionControllerComponent.IsTracked` _righthand)
    (set `self.IK_RightHand` (`KismetMathLibrary.MakeTransform` (.location (`KismetMathLibrary.ComposeTransforms` (`SceneComponent.K2_GetComponentToWorld` _righthand) (`KismetMathLibrary.InvertTransform` (`SceneComponent.K2_GetComponentToWorld` (`self.CharacterMesh0`))))) (`KismetMathLibrary.ComposeRotators` (`self.RotationOffset_RightHand`) (.rotation (`KismetMathLibrary.ComposeTransforms` (`SceneComponent.K2_GetComponentToWorld` _righthand) (`KismetMathLibrary.InvertTransform` (`SceneComponent.K2_GetComponentToWorld` (`self.CharacterMesh0`)))))) (.scale (`KismetMathLibrary.ComposeTransforms` (`SceneComponent.K2_GetComponentToWorld` _righthand) (`KismetMathLibrary.InvertTransform` (`SceneComponent.K2_GetComponentToWorld` (`self.CharacterMesh0`)))))))
    (`self.LogIKFunction` (`self.IK_RightHand`) "IK_RightHand")))

(fn `UpdateWaistTracker`
  (bind _waist (`self.Waist`))
  (bind _returnvalue (`MotionControllerComponent.IsTracked` _waist))
  (bind _returnvalue_2 (`SceneComponent.K2_GetComponentToWorld` _waist))
  (if (`self.blsCalibrated_Waist`)
    (`|ExecutionSequence`
      (:`then_0`
        (if _returnvalue
          (set `self.LastValidTransform_Waist` _returnvalue_2)))
      (:`then_1`
        (set `self.IK_Waist` (`KismetMathLibrary.TLerp` (`KismetMathLibrary.MakeTransform` (.location (`KismetMathLibrary.ComposeTransforms` (`KismetMathLibrary.SelectTransform` _returnvalue_2 (`self.LastValidTransform_Waist`) _returnvalue) (`KismetMathLibrary.InvertTransform` (`SceneComponent.K2_GetComponentToWorld` (`self.CharacterMesh0`))))) (.rotation (`KismetMathLibrary.ComposeTransforms` (`KismetMathLibrary.MakeTransform` (0.0 0.0 0.0) (`self.RotationOffset_Waist`)) (`KismetMathLibrary.MakeTransform` (0.0 0.0 0.0) (.rotation (`KismetMathLibrary.ComposeTransforms` (`KismetMathLibrary.SelectTransform` _returnvalue_2 (`self.LastValidTransform_Waist`) _returnvalue) (`KismetMathLibrary.InvertTransform` (`SceneComponent.K2_GetComponentToWorld` (`self.CharacterMesh0`)))))))) (.scale (`KismetMathLibrary.ComposeTransforms` (`KismetMathLibrary.SelectTransform` _returnvalue_2 (`self.LastValidTransform_Waist`) _returnvalue) (`KismetMathLibrary.InvertTransform` (`SceneComponent.K2_GetComponentToWorld` (`self.CharacterMesh0`)))))) (`self.IK_Waist`) (`KismetMathLibrary.FClamp` (* (* (`self.FilterStrength`) (`GameplayStatics.GetWorldDeltaSeconds`)) 60.0)))))
      (:`then_2`
        (`self.LogIKFunction` (`self.IK_Waist`) "IK_Waist")))))

(fn `UserConstructionScript`)